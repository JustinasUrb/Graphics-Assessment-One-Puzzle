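; BP_Keypad is a puzzle keypad that, on OpenDoor, destroys the completion door and a red light to reveal the green light behind it.
; Its collision volume enables input for the first-person character, and E toggles the W_KeypadScreen widget through a FlipFlop.
; Opening the widget sets UI-only input with a cursor, so E fails to close it.
; Leaving the volume disables input, removes all widgets and restores game controls.
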(event OnComponentBeginOverlap(Collision)
  (params (OverlappedComponent :type Primitive%20Component%20Object%20Reference) (OtherActor :type Actor%20Object%20Reference) (OtherComp :type Primitive%20Component%20Object%20Reference) (OtherBodyIndex :type Integer) (bFromSweep :type Boolean) (SweepResult :type Hit%20Result%20Structure%20%28by%20ref%29))
  ;[0.15 0.15 0.15 0.5] Logic for if player is within the keypad's zone of effect, where it enables player input for the keypad puzzle.
  (Utilities|Casting|CastToBP_FirstPersonCharacter OtherActor)
  (Input|EnableInput (Game|GetPlayerController 0)))

(event OnComponentEndOverlap(Collision)
  (params (OverlappedComponent :type Primitive%20Component%20Object%20Reference) (OtherActor :type Actor%20Object%20Reference) (OtherComp :type Primitive%20Component%20Object%20Reference) (OtherBodyIndex :type Integer))
  (bind _returnvalue (Game|GetPlayerController 0))
  ;[0.15 0.15 0.15 0.5] Logic for if player is within the keypad's zone of effect, where it enables player input for the keypad puzzle.
  (Utilities|Casting|CastToBP_FirstPersonCharacter OtherActor)
  (Input|DisableInput (Game|GetPlayerController 0))
  ;[0.15 0.15 0.15 0.5] If the player is outside the collision, or if the player presses 'E' (which doesn't work), the widget of the puzzle is removed, and proper player controls are restored.
  (Viewport|RemoveAllWidgets)
  (Input|SetInputModeGameOnly _returnvalue false)
  (Variables|/Script/Engine.PlayerController|SetbShowMouseCursor _returnvalue false))

(event Custom|Open%20Door
  ;[0.15 0.15 0.15 0.5] Once the correct combination is inputted, destroys the door to reach the end, as well as the red light to expose the green light behind (simple solution that was easier to implement than to change the colour).
  (Actor|DestroyActor (Variables|Default|GetCompletionDoor))
  (Actor|DestroyActor (Variables|Default|GetRemoveLight)))

(event Input|KeyboardEvents|E
  (params (Key :type Key%20Structure :default "None"))
  (bind _returnvalue (Game|GetPlayerController 0))
  (bind _returnvalue_2 (Game|GetPlayerController 0))
  ;[0.15 0.15 0.15 0.5] Should allow for the player to open the keypad, and close it with the press of the 'E' button. It works to open it, but not close it with this implementation.
  (:Pressed
    (Utilities|FlowControl|FlipFlop
      (:A
        ;[0.15 0.15 0.15 0.5] If the player presses 'E' within the collision zone, a widget is opened up (a screen with the keypad functionality), where it also disables user input outside the puzzle (as it becomes in focus of the widget).
        (bind _returnvalue_3 (UserInterface|CreateWidget "/Game/MyContent/MyBlueprints/W_KeypadScreen.W_KeypadScreen_C"))
        (UserInterface|Viewport|AddtoViewport _returnvalue_3 0)
        (Input|SetInputModeUIOnly _returnvalue_2 _returnvalue_3 "DoNotLock" false)
        (Variables|/Script/Engine.PlayerController|SetbShowMouseCursor _returnvalue_2 true))
      (:B
        ;[0.15 0.15 0.15 0.5] If the player is outside the collision, or if the player presses 'E' (which doesn't work), the widget of the puzzle is removed, and proper player controls are restored.
        (Viewport|RemoveAllWidgets)
        (Input|SetInputModeGameOnly _returnvalue false)
        (Variables|/Script/Engine.PlayerController|SetbShowMouseCursor _returnvalue false)))))

(fn ConstructionScript)